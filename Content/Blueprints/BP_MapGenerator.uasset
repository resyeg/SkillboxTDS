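; BP_MapGenerator is an actor meant to generate a room-based map from a seeded random stream, with generation still a stub.
; The construction script treats the NewSeed bool as an editor button that resets itself and rolls a random Seed, then always re-seeds the Stream from Seed.
; GenerateMap loops over RoomCount and checks for the first index, but creates nothing yet.
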(event `Generate Map`
  (for _index (range (`self.RoomCount`))
    (if (== _index 0)
      _)))

(fn `UserConstructionScript`
  (`|ExecutionSequence`
    (:`then_0`
      ;[1 1 1] On click "New Seed" get new random seed
      (if (`self.NewSeed`)
        (set `self.NewSeed` false)
        (set `self.Seed` (`KismetMathLibrary.RandomInteger` 900000))
        (`KismetMathLibrary.SetRandomStreamSeed` (`self.Stream`))))
    (:`then_1`
      ;[1 1 1] Manualy update sream with seed
      (`KismetMathLibrary.SetRandomStreamSeed` (`self.Stream`) (`self.Seed`)))))